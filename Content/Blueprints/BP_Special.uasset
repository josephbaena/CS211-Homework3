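; BP_Special is an actor Blueprint that sets up a customizable material on its static mesh, with no active gameplay logic.
; The Construction Script creates a dynamic instance of M_Special on element 0 and stores it as SpecialMaterial.
; It then passes the BaseColor, Metallic and Roughness variables to that instance, but every parameter name is left as None, so none target a named material parameter.
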(event `self.ReceiveBeginPlay`)

(event `self.ReceiveActorBeginOverlap`
  (params (OtherActor :type "Actor Object Reference")))

(event `self.ReceiveTick`
  (params (DeltaSeconds :type "Float (single-precision)")))

(fn `UserConstructionScript`
  (`|ExecutionSequence`
    (:`then_0`
      (bind _returnvalue (`PrimitiveComponent.CreateDynamicMaterialInstance` (`self.StaticMesh`) 0 "/Game/Materials/M_Special.M_Special"))
      (set `self.SpecialMaterial` _returnvalue))
    (:`then_1`
      (`MaterialInstanceDynamic.SetVectorParameterValue` (`self.SpecialMaterial`) "None" (`self.BaseColor`)))
    (:`then_2`
      (`MaterialInstanceDynamic.SetScalarParameterValue` (`self.SpecialMaterial`) "None" (`self.Metallic`)))
    (:`then_3`
      (`MaterialInstanceDynamic.SetScalarParameterValue` (`self.SpecialMaterial`) "None" (`self.Roughness`)))))